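; BP_Enemy is an enemy Blueprint whose chase and effect logic is present but disconnected, so BeginPlay and the construction script do nothing.
; One unreached loop re-issues an AI MoveTo toward the first BP_WarriorCharacter found every 0.2 seconds.
; Another unreached loop spawns a stunned particle in front of the enemy and plays a warrior hit sound every five seconds.
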(event `self.ReceiveBeginPlay`)

(fn `UserConstructionScript`)